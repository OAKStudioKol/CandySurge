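; BP_BaseCharacter is the base character Blueprint, mapping player input to aiming, firing, weapon cycling and sprinting.
; Aim start, cancel and completion share one FlipFlop, whose state a server RPC stores and messages to the AnimInstance.
; Fire only plays a montage on the combat component's equipped weapon mesh, with debug prints on its callbacks.
; Equip input cycles weapons through that component, while Left Shift directly changes walk speed.
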(fn `UserConstructionScript`)